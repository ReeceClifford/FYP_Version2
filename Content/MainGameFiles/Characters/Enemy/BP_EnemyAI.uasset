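; Enemy AI character that spots the main character through pawn sensing, turns to face them, chases and shoots.
; On sight it issues a move toward the player, spawns projectiles throttled by a delay-gated flag, and stores the player reference.
; TakeDamage reduces health, then calls IsDead and destroys the actor at zero.
; An unconnected leftover block would complete the player's matching quest and update the related NPC.
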(event `self.PawnSensing.OnSeePawn`
  (params (Pawn :type "Pawn Object Reference"))
  (bind _asbp_main_character (cast `/Game/MainGameFiles/Characters/BP_MainCharacter` Pawn))
  (`|ExecutionSequence`
    (:`then_0`
      (`self.K2_SetActorRotation` (`KismetMathLibrary.FindLookAtRotation` (`self.K2_GetActorLocation`) (`self.K2_GetActorLocation` _asbp_main_character)))
      (`|AIMoveTo` self (0.0 0.0 0.0) _asbp_main_character))
    (:`then_1`
      (if (`self.DelayShooting`)
        (`|SpawnActorFromClass` "/Game/MainGameFiles/Combat/BP_EnemyProjectile.BP_EnemyProjectile_C" (`SceneComponent.K2_GetComponentToWorld` (`self.ProjectileFire`)) "Undefined" "OverrideRootScale" null 0 0 null)
        (set `self.DelayShooting` false)
        (`KismetSystemLibrary.Delay` 1.0)
        (set `self.DelayShooting` true)))
    (:`then_2`
      (set `self.Player` _asbp_main_character))))

(event `TakeDamage`
  (params (DamageToTake :type "Float (double-precision)"))
  (bind _output_get (set `self.EnemyHealth` (- (`self.EnemyHealth`) DamageToTake)))
  (if (<= _output_get 0.0)
    (`|ExecutionSequence`
      (:`then_0`
        (`self.IsDead`))
      (:`then_1`
        (`self.K2_DestroyActor`)))))

(fn `UserConstructionScript`)