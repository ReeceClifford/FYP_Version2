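; BP_Spawner spawns a quest enemy and completes the linked quest when that enemy dies.
; SpawnEnemy stores the requester, spawns a BP_EnemyAI at its Sphere with configured health and tree, then binds to its IsDead event.
; On death, it completes any active quest referencing this spawner, then updates matching NPC_CharacterOne actors by quest name, changing their tree and playing a completion sound.
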(event `SpawnEnemy`
  (params (WhoSpawned :type "/Game/MainGameFiles/Characters/BP_MainCharacter Object Reference"))
  (set `self.Who Spawned` WhoSpawned)
  (bind _returnvalue (`|SpawnActorFromClass` "/Game/MainGameFiles/Characters/Enemy/BP_EnemyAI.BP_EnemyAI_C" (`KismetMathLibrary.MakeTransform` (`SceneComponent.K2_GetComponentLocation` (`self.Sphere`)) (struct :`Yaw` 180.0)) "AdjustIfPossibleButAlwaysSpawn" "OverrideRootScale" null (`self.Enemy Health`) (`self.Tree To Change To`) null))
  (bind _output_get (set `self.Enemy Spawned` _returnvalue))
  (add `/Game/MainGameFiles/Characters/Enemy/BP_EnemyAI.IsDead` _output_get (delegate `SpawnedEnemyDead`)))

(event `SpawnedEnemyDead`
  (for _array_element (`/Game/MainGameFiles/Characters/BP_MainCharacter.ActiveQuests` (`self.Who Spawned`))
    (bind (_questinfo_questname _questinfo_questdescription _questinfo_actorreference) (break `/Game/MainGameFiles/Quests/s_QuestInfo` (`/Game/MainGameFiles/UI/wbp_Quest.QuestInfo` _array_element)))
    (if (== self _questinfo_actorreference)
      (`/Game/MainGameFiles/Characters/BP_MainCharacter.QuestComplete` (`self.Who Spawned`) _array_element)
      (bind _outactors (`GameplayStatics.GetAllActorsOfClass` "/Game/MainGameFiles/Characters/NPCs/NPC_CharacterOne.NPC_CharacterOne_C"))
      (for _array_element_2 _outactors
        (bind _quest_ref_questname (break `/Game/MainGameFiles/Quests/s_QuestInfo` (`/Game/MainGameFiles/Characters/NPCs/NPC_CharacterOne.Quest Ref` _array_element_2)))
        (if (== _questinfo_questname _quest_ref_questname)
          (`/Game/MainGameFiles/Characters/NPCs/NPC_CharacterOne.ChangeTreeAfterEvent` _array_element_2 (`self.Tree To Change To`))
          (`/Game/MainGameFiles/Characters/NPCs/NPC_CharacterOne.QuestComplete` _array_element_2)
          (`GameplayStatics.PlaySound2D` "/Game/MainGameFiles/Sounds/Complete.Complete" 1.0 1.0 0.0 null null))))))

(fn `UserConstructionScript`)