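; Location trigger actor that completes quests whose objective is the player reaching this spot.
; When BP_MainCharacter overlaps the box, it checks the character's active quests for any whose ActorReference is this actor and completes them.
; It then finds every NPC_CharacterOne with a matching quest name, switches its tree to TreeToChangeTo and marks its quest complete.
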(event `self.Box.OnComponentBeginOverlap`
  (params (OverlappedComponent :type "PrimitiveComponent Object Reference") (OtherActor :type "Actor Object Reference") (OtherComp :type "PrimitiveComponent Object Reference") (OtherBodyIndex :type Integer) (bFromSweep :type Boolean) (SweepResult :type "HitResult Structure (by ref)"))
  (bind _asbp_main_character (cast `/Game/MainGameFiles/Characters/BP_MainCharacter` OtherActor))
  (for _array_element (`/Game/MainGameFiles/Characters/BP_MainCharacter.ActiveQuests` _asbp_main_character)
    (bind (_questinfo_questname _questinfo_questdescription _questinfo_actorreference) (break `/Game/MainGameFiles/QuestInfo` (`/Game/MainGameFiles/BP_Quest.QuestInfo` _array_element)))
    (if (== self _questinfo_actorreference)
      (`/Game/MainGameFiles/Characters/BP_MainCharacter.QuestComplete` _asbp_main_character _array_element)
      (bind _outactors (`GameplayStatics.GetAllActorsOfClass` "/Game/MainGameFiles/Characters/NPCs/NPC_CharacterOne.NPC_CharacterOne_C"))
      (for _array_element_2 _outactors
        (bind _quest_ref_questname (break `/Game/MainGameFiles/QuestInfo` (`/Game/MainGameFiles/Characters/NPCs/NPC_CharacterOne.Quest Ref` _array_element_2)))
        (if (== _questinfo_questname _quest_ref_questname)
          (`/Game/MainGameFiles/Characters/NPCs/NPC_CharacterOne.ChangeTreeAfterEvent` _array_element_2 (`self.TreeToChangeTo`))
          (`/Game/MainGameFiles/Characters/NPCs/NPC_CharacterOne.QuestComplete` _array_element_2))))))

(fn `UserConstructionScript`)